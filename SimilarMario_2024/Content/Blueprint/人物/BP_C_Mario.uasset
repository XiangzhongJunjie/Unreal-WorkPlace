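; Player Mario character for a side-scroller: moves and jumps along X, with Tick pinning Y to 800 while alive.
; Overlapping a "蘑菇" (mushroom) sets a powered-up flag and grows the capsule via timeline.
; A "蘑菇怪" (mushroom monster) hit passes through a delay-reset DoOnce, either shrinking the powered-up character or triggering death.
; Death blocks input, pops the character upward, slides it along Y, then destroys it.
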(event `self.ReceiveTick`
  (params (DeltaSeconds :type "Float (single-precision)"))
  (bind (_returnvalue_x _returnvalue_y _returnvalue_z) (`KismetMathLibrary.BreakVector` (`self.K2_GetActorLocation`)))
  (if (not (`self.角色是否死亡`))
    (`self.K2_SetActorLocation` (`KismetMathLibrary.MakeVector` _returnvalue_x 800.0 _returnvalue_z))))

(event `InputAxis|左右移动`
  (params (AxisValue :type "Float (single-precision)"))
  (if (not (`self.角色是否死亡`))
    (`self.AddMovementInput` (1.0 0.0 0.0) AxisValue)
    (if (> AxisValue 0.0)
      (`SceneComponent.K2_SetRelativeRotation` (`self.Mesh`) (struct :`Yaw` -90.0) false false)
      (elif (< AxisValue 0.0)
        (`SceneComponent.K2_SetRelativeRotation` (`self.Mesh`) (struct :`Yaw` 90.0) false false)))))

(event `InputAction|跳跃`
  (params (Key :type "Key Structure"))
  (:`Pressed`
    (if (not (`self.角色是否死亡`))
      (`self.Jump`)))
  (:`Released`
    (`self.StopJumping`)))

(event `self.CapsuleComponent.OnComponentBeginOverlap`
  (params (OverlappedComponent :type "PrimitiveComponent Object Reference") (OtherActor :type "Actor Object Reference") (OtherComp :type "PrimitiveComponent Object Reference") (OtherBodyIndex :type Integer) (bFromSweep :type Boolean) (SweepResult :type "HitResult Structure (by ref)"))
  (if (`self.ActorHasTag` OtherActor "蘑菇")
    (`self.K2_DestroyActor` OtherActor)
    (set `self.吃过了蘑菇` true)
    (bind (_direction `_变化的过程`) (`Timeline|让角色快速的变大缩小` :!via `PlayFromStart` :!label _label)
      (:`Update`
        (`SceneComponent.SetRelativeScale3D` (`self.CapsuleComponent`) (`KismetMathLibrary.VLerp` (0.6 0.6 0.6) (1.0 1.0 1.0) `_变化的过程`)))
      (:`Finished`
        (`KismetSystemLibrary.Delay` 1.0)
        (goto _label_2 :!via `Reset`)))
    (elif (`self.ActorHasTag` OtherActor "蘑菇怪")
      (`/Engine/EditorBlueprintResources/StandardMacros.DoOnce` false :!label _label_2
        (:`Completed`
          (if (`self.吃过了蘑菇`)
            (set `self.吃过了蘑菇` false)
            (goto _label :!via `ReverseFromEnd`)
            (else
              (`self.角色死亡`)
              (`KismetSystemLibrary.Delay` 1.0)
              (goto _label_2 :!via `Reset`))))))))

(event `角色死亡`
  (bind (_returnvalue_x _returnvalue_y _returnvalue_z) (`KismetMathLibrary.BreakVector` (`self.K2_GetActorLocation`)))
  (set `self.角色是否死亡` true)
  (`SceneComponent.K2_SetRelativeRotation` :`self` (`self.Mesh`))
  (`KismetSystemLibrary.Delay` 0.2)
  (set `CharacterMovementComponent.JumpZVelocity` 1000.0 (`self.CharacterMovement`))
  (`self.Jump`)
  (bind (_direction `_新建轨道_0`) (`Timeline|让角色在Y轴方向有速度` :!via `PlayFromStart`)
    (:`Update`
      (`self.K2_SetActorLocation` (`KismetMathLibrary.MakeVector` _returnvalue_x (`KismetMathLibrary.Lerp` 800.0 1400.0 `_新建轨道_0`) _returnvalue_z)))
    (:`Finished`
      (`KismetSystemLibrary.Delay` 2.0)
      (`self.K2_DestroyActor`))))

(fn `UserConstructionScript`)