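; Mushroom item actor that slides back and forth along the world X axis.
; Tick offsets its location by a signed per-frame speed, without delta-time scaling.
; An overlap on its collision component flips that speed's sign, with a DoOnce and one-second Delay preventing rapid repeated reversals.
; Collision hits only print a debug string.
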(event `self.ReceiveTick`
  (params (DeltaSeconds :type "Float (single-precision)"))
  (bind (_returnvalue_x _returnvalue_y _returnvalue_z) (`KismetMathLibrary.BreakVector` (`self.K2_GetActorLocation`)))
  (`self.K2_SetActorLocation` (`KismetMathLibrary.MakeVector` (+ (`self.蘑菇的移动方向与速度`) _returnvalue_x) _returnvalue_y _returnvalue_z)))

(event `self.蘑菇的碰撞检测.OnComponentHit`
  (params (HitComponent :type "PrimitiveComponent Object Reference") (OtherActor :type "Actor Object Reference") (OtherComp :type "PrimitiveComponent Object Reference") (NormalImpulse :type "Vector Structure") (Hit :type "HitResult Structure (by ref)"))
  (`KismetSystemLibrary.PrintString` "Hello"))

(event `self.蘑菇的碰撞检测.OnComponentBeginOverlap`
  (params (OverlappedComponent :type "PrimitiveComponent Object Reference") (OtherActor :type "Actor Object Reference") (OtherComp :type "PrimitiveComponent Object Reference") (OtherBodyIndex :type Integer) (bFromSweep :type Boolean) (SweepResult :type "HitResult Structure (by ref)"))
  (`/Engine/EditorBlueprintResources/StandardMacros.DoOnce` false :!label _label
    (:`Completed`
      (if (== (`self.蘑菇的移动方向与速度`) 10.0)
        (set `self.蘑菇的移动方向与速度` -10.0)
        (`KismetSystemLibrary.Delay` 1.0)
        (goto _label :!via `Reset`)
        (else
          (set `self.蘑菇的移动方向与速度` 10.0)
          (`KismetSystemLibrary.Delay` 1.0)
          (goto _label :!via `Reset`))))))

(fn `UserConstructionScript`)